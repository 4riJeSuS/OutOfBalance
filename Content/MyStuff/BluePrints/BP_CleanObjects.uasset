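; BP_CleanObjects is an interactable actor whose mesh comes from an ObjectMesh variable set in the construction script, and which removes itself on interaction.
; It enables input from the first player controller on BeginPlay, so the interact action fires without any overlap or proximity check.
; The first trigger plays a timeline, which on finishing scales the mesh by its track value and destroys the actor.
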(event `self.ReceiveBeginPlay`
  (`self.EnableInput` (`GameplayStatics.GetPlayerController` 0)))

(event `EnhancedInput|/Game/Variant_SideScrolling/Input/Actions/IA_Interact_`
  (params (ActionValue :type Boolean) (ElapsedSeconds :type "Float (double-precision)") (TriggeredSeconds :type "Float (double-precision)") (InputAction :type "InputAction Object Reference" :default "/Game/Variant_SideScrolling/Input/Actions/IA_Interact_.IA_Interact_"))
  (:`Triggered`
    (`KismetSystemLibrary.PrintString` "Hello")
    (`/Engine/EditorBlueprintResources/StandardMacros.DoOnce` false
      (:`Completed`
        (bind (_direction _newtrack_0) (`Timeline|Timeline`)
          (:`Finished`
            (`SceneComponent.SetRelativeScale3D` (`self.StaticMesh`) (`KismetMathLibrary.MakeVector` _newtrack_0 _newtrack_0 _newtrack_0))
            (`self.K2_DestroyActor`)))))))

(fn `UserConstructionScript`
  (`StaticMeshComponent.SetStaticMesh` (`self.StaticMesh`) (`self.ObjectMesh`)))