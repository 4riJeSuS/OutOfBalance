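; BP_Altar is an altar actor that reveals a photo held in a child actor component.
; The construction script creates a dynamic fade material on the child BP_PhotoA's mesh and sets its opacity to zero.
; The ActivateFade event plays a timeline that drives that opacity, and each update also detaches PhotoA in world space and makes it visible.
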(event `self.ReceiveBeginPlay`)

(event `ActivateFade`
  (bind _photoa (`self.PhotoA`))
  (bind (_direction _alfha) (`Timeline|TimelineFade`)
    (:`Update`
      (`MaterialInstanceDynamic.SetScalarParameterValue` (`self.MaterialDyn_Ref`) "Opacity" _alfha)
      (`SceneComponent.K2_DetachFromComponent` _photoa "KeepWorld" "KeepWorld" "KeepRelative" true)
      (`SceneComponent.SetVisibility` _photoa true false))))

(fn `UserConstructionScript`
  (bind _asbp_photo_a (cast `/Game/MyStuff/BluePrints/BP_PhotoA` (`ChildActorComponent.ChildActor` (`self.PhotoA`))))
  (bind _returnvalue (`PrimitiveComponent.CreateDynamicMaterialInstance` (`/Game/MyStuff/BluePrints/BP_PhotoA.SM_Photo` _asbp_photo_a) 0 "/Game/MyStuff/Textures/M_Photo_Fade.M_Photo_Fade" "None"))
  (bind _output_get (set `self.MaterialDyn_Ref` _returnvalue))
  (`MaterialInstanceDynamic.SetScalarParameterValue` _output_get "Opacity" 0.0))