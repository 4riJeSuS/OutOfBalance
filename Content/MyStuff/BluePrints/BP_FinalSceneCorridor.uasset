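; BP_FinalSceneCorridor is a one-shot overlap trigger that runs a scripted corridor sequence for the final scene.
; When BP_Player enters, it disables movement, stops the hall voices timer and, after delays, plays a 2D sound.
; It flashes the hall spotlights red-orange, switches lights off with a pale blue color, then fires the trigger component on the hall's rotative doors.
; Finally it restores walking movement and destroys itself.
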(event `self.ReceiveActorBeginOverlap`
  (params (OtherActor :type "Actor Object Reference"))
  (bind _asbp_player (cast `/Game/MyStuff/PlayerSetting/BP_Player` OtherActor))
  (bind _charactermovement (`Character.CharacterMovement` _asbp_player))
  (`CharacterMovementComponent.DisableMovement` _charactermovement)
  (`KismetSystemLibrary.K2_ClearAndInvalidateTimerHandle` (`/Game/MyStuff/BluePrints/BP_HallInte.TimerVoicesHandle` (`self.RefHallInte`)))
  (`KismetSystemLibrary.Delay` 4.0)
  (`GameplayStatics.PlaySound2D` "/Game/MyStuff/Sounds/SchoolHall/SchoolHall8.SchoolHall8" 1.0 1.0 0.0 null null)
  (`KismetSystemLibrary.Delay` 5.0)
  (for _array_element (`self.HallLights`)
    (bind _spotlightcomponent (`SpotLight.SpotLightComponent` _array_element))
    (`LightComponent.SetIntensity` _spotlightcomponent 5000.0)
    (`LightComponent.SetLightColor` _spotlightcomponent (struct :`R` 1.0 :`G` 0.132868 :`B` 0.01033 :`A` 1.0) true))
  (`KismetSystemLibrary.Delay` 1.0)
  (for _array_element_2 _
    (bind _spotlightcomponent_2 (`SpotLight.SpotLightComponent` _array_element_2))
    (`LightComponent.SetIntensity` _spotlightcomponent_2 0.0)
    (`LightComponent.SetLightColor` _spotlightcomponent_2 (struct :`R` 0.566514 :`G` 0.729385 :`B` 0.869792 :`A` 1.0) true))
  (for _array_element_3 (`self.HallDoors`)
    (bind _asbp_rrotative_door (cast `/Game/MyStuff/BluePrints/BP_RRotativeDoor` _array_element_3))
    (`TriggerComponent.Trigger` (`self.GetComponentByClass` _asbp_rrotative_door "/Script/OutOfBalance.TriggerComponent") true))
  (`CharacterMovementComponent.SetMovementMode` _charactermovement "MOVE_Walking" 0)
  (`self.K2_DestroyActor`))

(fn `UserConstructionScript`)