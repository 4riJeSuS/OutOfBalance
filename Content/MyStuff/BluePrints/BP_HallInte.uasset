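; BP_HallInte is a hallway trigger that closes doors and starts recurring voice sounds when the player enters.
; The first overlap passes a DoOnce, casts to BP_Player, calls Trigger with false on its Trigger reference and starts a looping timer at TimeBSounds intervals.
; The timer plays SC_HallVoices in 2D, with a DoOnce and Delay limiting how often it repeats.
; DoOnce precedes the cast, so a non-player overlap also consumes it.
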(event `TimesItPlays`
  (`/Engine/EditorBlueprintResources/StandardMacros.DoOnce` false :!label _label
    (:`Completed`
      (`GameplayStatics.PlaySound2D` "/Game/MyStuff/Sounds/SC_HallVoices.SC_HallVoices" 1.0 1.0 0.0 null null)
      (`KismetSystemLibrary.Delay` 2.0)
      (goto _label :!via `Reset`))))

(event `self.ReceiveActorBeginOverlap`
  (params (OtherActor :type "Actor Object Reference"))
  ; Fechar portas
  (`/Engine/EditorBlueprintResources/StandardMacros.DoOnce` false
    (:`Completed`
      (cast `/Game/MyStuff/PlayerSetting/BP_Player` OtherActor)
      (`TriggerComponent.Trigger` (`self.Trigger`) false)
      (bind _returnvalue (`KismetSystemLibrary.K2_SetTimer` null "TimesItPlays" (`self.TimeBSounds`) true))
      (set `self.TimerVoicesHandle` _returnvalue))))

(fn `UserConstructionScript`)