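; BP_ClearObjects is an actor that updates the player's inventory and the room manager when it is destroyed.
; Its construction script applies the MeshObject variable to the static mesh, so each instance can have its own look.
; On Destroyed, it removes ItemName from the OutOfBalanceCharacter's inventory, then calls RemovedPlates on the BP_M2RoomManager found in the level.
; The manager is notified only if the player cast succeeds.
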(event `self.ReceiveDestroyed`
  (bind _asout_of_balance_character (cast `OutOfBalanceCharacter` (`GameplayStatics.GetPlayerCharacter` 0)))
  (`KismetArrayLibrary.Array_RemoveItem` (`OutOfBalanceCharacter.inventory` _asout_of_balance_character) (`self.itemName`))
  (bind _returnvalue (`GameplayStatics.GetActorOfClass` "/Game/MyStuff/BluePrints/BP_M2RoomManager.BP_M2RoomManager_C"))
  (`/Game/MyStuff/BluePrints/BP_M2RoomManager.RemovedPlates` _returnvalue))

(fn `UserConstructionScript`
  (`StaticMeshComponent.SetStaticMesh` (`self.StaticMesh`) (`self.MeshObject`)))