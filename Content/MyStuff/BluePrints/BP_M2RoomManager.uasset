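; BP_M2RoomManager manages a room's audio as the objects in it are cleared.
; On begin play it counts all BP_ClearObjects actors, and the first OutOfBalanceCharacter overlap with TriggerRoom fades in the music.
; Each RemovedPlates call decrements the count, scales music volume to the fraction remaining, and prints the count.
; When none remain, a camera shutter sound plays after a short delay.
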(event `self.ReceiveBeginPlay`
  (bind _outactors (`GameplayStatics.GetAllActorsOfClass` "/Game/MyStuff/BluePrints/BP_ClearObjects.BP_ClearObjects_C"))
  (bind _output_get (set `self.NumberofObjects` (`KismetArrayLibrary.Array_Length` _outactors)))
  (set `self.TotalNumberofObjects` _output_get))

(event `RemovedPlates`
  (bind _output_get (set `self.NumberofObjects` (- (`self.NumberofObjects`) 1)))
  (`AudioComponent.SetVolumeMultiplier` (`self.Music`) (/ _output_get (`KismetMathLibrary.Conv_IntToDouble` (`self.TotalNumberofObjects`))))
  (`KismetSystemLibrary.PrintString` (`KismetStringLibrary.Conv_IntToString` _output_get))
  (`/Engine/EditorBlueprintResources/StandardMacros.CompareInt` _output_get
    (:`==`
      (`KismetSystemLibrary.Delay` 1.0)
      (`GameplayStatics.PlaySound2D` "/Engine/VREditor/Sounds/UI/Camera_Shutter.Camera_Shutter" 1.0 1.0 0.0 null null))))

(event `self.TriggerRoom.OnComponentBeginOverlap`
  (params (OverlappedComponent :type "PrimitiveComponent Object Reference") (OtherActor :type "Actor Object Reference") (OtherComp :type "PrimitiveComponent Object Reference") (OtherBodyIndex :type Integer) (bFromSweep :type Boolean) (SweepResult :type "HitResult Structure (by ref)"))
  (cast `OutOfBalanceCharacter` OtherActor)
  (`/Engine/EditorBlueprintResources/StandardMacros.DoOnce` false
    (:`Completed`
      (`AudioComponent.FadeIn` (`self.Music`) 2.0 1.0 0.0 "Linear")
      (`GameplayStatics.PlaySound2D` null 1.0 1.0 0.0 null null))))

(fn `UserConstructionScript`)