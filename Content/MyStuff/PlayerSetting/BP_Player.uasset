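; BP_Player is a player pawn with Enhanced Input movement and an angled camera that turns in 45-degree steps.
; Q and E step TargetYaw, and Tick eases the CameraBoom's relative rotation toward it at a fixed downward pitch.
; Separate Q and E handlers also set control rotation from TargetYaw, whose yaw orients IA_Move's forward and right movement.
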(event `EnhancedInput|/Game/Input/Actions/IA_Move`
  (params (ActionValue :type "Vector2D Structure") (ElapsedSeconds :type "Float (double-precision)") (TriggeredSeconds :type "Float (double-precision)") (InputAction :type "InputAction Object Reference" :default "/Game/Input/Actions/IA_Move.IA_Move"))
  (bind (_x _y) (`KismetMathLibrary.BreakVector2D` ActionValue))
  (bind _returnvalue (`KismetMathLibrary.MakeRotator` 0.0 0.0 (.yaw (`Controller.GetControlRotation` (`GameplayStatics.GetPlayerController` 0)))))
  (:`Triggered`
    (`self.AddMovementInput` (`KismetMathLibrary.GetForwardVector` _returnvalue) _y)
    (`self.AddMovementInput` (`KismetMathLibrary.GetRightVector` _returnvalue) _x)))

(event `self.ReceiveTick`
  (params (DeltaSeconds :type "Float (single-precision)"))
  (`SceneComponent.K2_SetRelativeRotation` (`self.CameraBoom`) (`KismetMathLibrary.RInterpTo` (`SceneComponent.RelativeRotation` (`self.CameraBoom`)) (`KismetMathLibrary.MakeRotator` 0.0 -45.0 (`self.TargetYaw`)) (`GameplayStatics.GetWorldDeltaSeconds`) 5.0) false false))

(event `Key|Q`
  (params (Key :type "Key Structure"))
  (:`Pressed`
    (`Controller.SetControlRotation` (`GameplayStatics.GetPlayerController` 0) (`KismetMathLibrary.MakeRotator` 0.0 -45.0 (`self.TargetYaw`)))))

(event `Key|E`
  (params (Key :type "Key Structure"))
  (:`Pressed`
    (`Controller.SetControlRotation` (`GameplayStatics.GetPlayerController` 0) (`KismetMathLibrary.MakeRotator` 0.0 -45.0 (`self.TargetYaw`)))))

(event `Key|Q`
  (params (Key :type "Key Structure"))
  (:`Pressed`
    (set `self.TargetYaw` (+ (`self.TargetYaw`) -45.0))))

(event `Key|E`
  (params (Key :type "Key Structure"))
  (:`Pressed`
    (set `self.TargetYaw` (+ (`self.TargetYaw`) 45.0))))

(fn `UserConstructionScript`
  (`parent.UserConstructionScript`))